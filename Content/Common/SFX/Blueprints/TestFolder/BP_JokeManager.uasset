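; Test-folder sound manager that stages three jokes with 2D player voice and crowd SFX on timed delays.
; Start events play intro or setup lines over applause; only StartJoke01 chains into its End event.
; End events branch on IsJokeGood: good punchlines get FlipFlop-alternated laughter plus applause, bad ones get booing and screams on every other run.
; Jokes 2 and 3 reuse some Joke01 clips.
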(event Custom|End_Joke03
  ;[0.04254 0.2873 0.4896] End_Joke03
  (if (Variables|Default|GetIsJokeGood?)
    (bind _returnvalue (Audio|SpawnSound2D "/Game/Common/SFX/Player/SFX_Player_Joke03_GoodPunchline.SFX_Player_Joke03_GoodPunchline" 2.0 1.0 0.0 0 false false))
    (Components|Activation|SetActive _returnvalue true false)
    (Utilities|FlowControl|Delay 2.0)
    (Utilities|FlowControl|FlipFlop
      (:A
        (bind _returnvalue_2 (Audio|SpawnSound2D "/Game/Common/SFX/Crowd/SFX_Crowd_Large_Laughter.SFX_Crowd_Large_Laughter" 1.0 1.0 0.0 0 false false))
        (Components|Activation|SetActive _returnvalue_2 true false))
      (:B
        (bind _returnvalue_3 (Audio|SpawnSound2D "/Game/Common/SFX/Crowd/SFX_Crowd_Medium_Laughter.SFX_Crowd_Medium_Laughter" 1.0 1.0 0.0 0 false false))
        (Components|Activation|SetActive _returnvalue_3 true false)))
    (bind _returnvalue_4 (Audio|SpawnSound2D "/Game/Common/SFX/Crowd/SFX_Crowd_Medium_Applause.SFX_Crowd_Medium_Applause" 1.0 1.0 0.0 0 false false))
    (Components|Activation|SetActive _returnvalue_4 true false)
    (else
      (bind _returnvalue_5 (Audio|SpawnSound2D "/Game/Common/SFX/Player/SFX_Player_Joke03_BadPunchline.SFX_Player_Joke03_BadPunchline" 2.0 1.0 0.0 0))
      (Components|Activation|SetActive _returnvalue_5 true false)
      (Utilities|FlowControl|Delay 3.0)
      (Utilities|FlowControl|FlipFlop
        (:A
          (bind _returnvalue_6 (Audio|SpawnSound2D "/Game/Common/SFX/Crowd/SFX_Crowd_Large_Booing.SFX_Crowd_Large_Booing" 1.0 1.0 0.0 0 false false))
          (Components|Activation|SetActive _returnvalue_6 true false)
          (bind _returnvalue_7 (Audio|SpawnSound2D "/Game/Common/SFX/Crowd/SFX_Crowd_Large_AngryScreams.SFX_Crowd_Large_AngryScreams" 1.0 1.0 0.0 0 false false))
          (Components|Activation|SetActive _returnvalue_7 true false)
          (Utilities|FlowControl|Delay 5.0)
          (Components|Activation|ToggleActive _returnvalue_7))))))

(event Custom|StartJoke03
  ;[1 1 1] Start_Joke03
  (bind _returnvalue (Audio|SpawnSound2D "/Game/Common/SFX/Player/SFX_Player_Joke03_Setup.SFX_Player_Joke03_Setup" 1.0 1.0 0.0 0 false false))
  (Components|Activation|SetActive _returnvalue true false)
  (Utilities|FlowControl|Delay 1.0)
  (bind _returnvalue_2 (Audio|SpawnSound2D "/Game/Common/SFX/Crowd/SFX_Crowd_Large_Applause.SFX_Crowd_Large_Applause" 1.0 1.0 0.0 0 false false))
  (Components|Activation|SetActive _returnvalue_2 true false)
  (bind _returnvalue_3 (Audio|SpawnSound2D "/Game/Common/SFX/Crowd/SFX_Crowd_Medium_Applause.SFX_Crowd_Medium_Applause" 1.0 1.0 0.0 0 false false))
  (Components|Activation|SetActive _returnvalue_3 true false)
  (Utilities|FlowControl|Delay 1e+01)
  (bind _returnvalue_4 (Audio|SpawnSound2D "/Game/Common/SFX/Player/SFX_Player_Joke01_Setup.SFX_Player_Joke01_Setup" 2.0 1.0 0.0 0))
  (Components|Activation|SetActive _returnvalue_4 true false))

(event Custom|EndJoke01
  ;[0.04254 0.2873 0.4896] End_Joke01
  (if (Variables|Default|GetIsJokeGood?)
    (bind _returnvalue (Audio|SpawnSound2D "/Game/Common/SFX/Player/SFX_Player_Joke01_GoodPunchline.SFX_Player_Joke01_GoodPunchline" 2.0 1.0 0.0 0 false false))
    (Components|Activation|SetActive _returnvalue true false)
    (Utilities|FlowControl|Delay 2.0)
    (Utilities|FlowControl|FlipFlop
      (:A
        (bind _returnvalue_2 (Audio|SpawnSound2D "/Game/Common/SFX/Crowd/SFX_Crowd_Large_Laughter.SFX_Crowd_Large_Laughter" 1.0 1.0 0.0 0 false false))
        (Components|Activation|SetActive _returnvalue_2 true false))
      (:B
        (bind _returnvalue_3 (Audio|SpawnSound2D "/Game/Common/SFX/Crowd/SFX_Crowd_Medium_Laughter.SFX_Crowd_Medium_Laughter" 1.0 1.0 0.0 0 false false))
        (Components|Activation|SetActive _returnvalue_3 true false)))
    (bind _returnvalue_4 (Audio|SpawnSound2D "/Game/Common/SFX/Crowd/SFX_Crowd_Medium_Applause.SFX_Crowd_Medium_Applause" 1.0 1.0 0.0 0 false false))
    (Components|Activation|SetActive _returnvalue_4 true false)
    (else
      (bind _returnvalue_5 (Audio|SpawnSound2D "/Game/Common/SFX/Player/SFX_Player_Joke01_BadPunchline.SFX_Player_Joke01_BadPunchline" 2.0 1.0 0.0 0))
      (Components|Activation|SetActive _returnvalue_5 true false)
      (Utilities|FlowControl|Delay 3.0)
      (Utilities|FlowControl|FlipFlop
        (:A
          (bind _returnvalue_6 (Audio|SpawnSound2D "/Game/Common/SFX/Crowd/SFX_Crowd_Large_Booing.SFX_Crowd_Large_Booing" 1.0 1.0 0.0 0 false false))
          (Components|Activation|SetActive _returnvalue_6 true false)
          (bind _returnvalue_7 (Audio|SpawnSound2D "/Game/Common/SFX/Crowd/SFX_Crowd_Large_AngryScreams.SFX_Crowd_Large_AngryScreams" 1.0 1.0 0.0 0 false false))
          (Components|Activation|SetActive _returnvalue_7 true false)
          (Utilities|FlowControl|Delay 5.0)
          (Components|Activation|ToggleActive _returnvalue_7))))))

(event Custom|StartJoke01
  ;[1 1 1] Start_Joke01
  (bind _returnvalue (Audio|SpawnSound2D "/Game/Common/SFX/Ambient/SFX_Ambient_IntroJingle.SFX_Ambient_IntroJingle" 1.0 1.0 0.0 0 false false))
  (Components|Activation|SetActive _returnvalue true false)
  (Utilities|FlowControl|Delay 1.0)
  (bind _returnvalue_2 (Audio|SpawnSound2D "/Game/Common/SFX/Crowd/SFX_Crowd_Large_Applause.SFX_Crowd_Large_Applause" 1.0 1.0 0.0 0 false false))
  (Components|Activation|SetActive _returnvalue_2 true false)
  (bind _returnvalue_3 (Audio|SpawnSound2D "/Game/Common/SFX/Crowd/SFX_Crowd_Medium_Applause.SFX_Crowd_Medium_Applause" 1.0 1.0 0.0 0 false false))
  (Components|Activation|SetActive _returnvalue_3 true false)
  (Utilities|FlowControl|Delay 1e+01)
  (bind _returnvalue_4 (Audio|SpawnSound2D "/Game/Common/SFX/Player/SFX_Player_Joke01_Setup.SFX_Player_Joke01_Setup" 2.0 1.0 0.0 0))
  (Components|Activation|SetActive _returnvalue_4 true false)
  (Utilities|FlowControl|Delay 4.0)
  (CallFunction|EndJoke01))

(event Custom|EndJoke02
  ;[0.04254 0.2873 0.4896] End_Joke02
  (if (Variables|Default|GetIsJokeGood?)
    (bind _returnvalue (Audio|SpawnSound2D "/Game/Common/SFX/Player/SFX_Player_Joke02_GoodPunchline.SFX_Player_Joke02_GoodPunchline" 2.0 1.0 0.0 0 false false))
    (Components|Activation|SetActive _returnvalue true false)
    (Utilities|FlowControl|Delay 2.0)
    (Utilities|FlowControl|FlipFlop
      (:A
        (bind _returnvalue_2 (Audio|SpawnSound2D "/Game/Common/SFX/Crowd/SFX_Crowd_Large_Laughter.SFX_Crowd_Large_Laughter" 1.0 1.0 0.0 0 false false))
        (Components|Activation|SetActive _returnvalue_2 true false))
      (:B
        (bind _returnvalue_3 (Audio|SpawnSound2D "/Game/Common/SFX/Crowd/SFX_Crowd_Medium_Laughter.SFX_Crowd_Medium_Laughter" 1.0 1.0 0.0 0 false false))
        (Components|Activation|SetActive _returnvalue_3 true false)))
    (bind _returnvalue_4 (Audio|SpawnSound2D "/Game/Common/SFX/Crowd/SFX_Crowd_Medium_Applause.SFX_Crowd_Medium_Applause" 1.0 1.0 0.0 0 false false))
    (Components|Activation|SetActive _returnvalue_4 true false)
    (else
      (bind _returnvalue_5 (Audio|SpawnSound2D "/Game/Common/SFX/Player/SFX_Player_Joke01_BadPunchline.SFX_Player_Joke01_BadPunchline" 2.0 1.0 0.0 0))
      (Components|Activation|SetActive _returnvalue_5 true false)
      (Utilities|FlowControl|Delay 3.0)
      (Utilities|FlowControl|FlipFlop
        (:A
          (bind _returnvalue_6 (Audio|SpawnSound2D "/Game/Common/SFX/Crowd/SFX_Crowd_Large_Booing.SFX_Crowd_Large_Booing" 1.0 1.0 0.0 0 false false))
          (Components|Activation|SetActive _returnvalue_6 true false)
          (bind _returnvalue_7 (Audio|SpawnSound2D "/Game/Common/SFX/Crowd/SFX_Crowd_Large_AngryScreams.SFX_Crowd_Large_AngryScreams" 1.0 1.0 0.0 0 false false))
          (Components|Activation|SetActive _returnvalue_7 true false)
          (Utilities|FlowControl|Delay 5.0)
          (Components|Activation|ToggleActive _returnvalue_7))))))

(event Custom|StartJoke02
  ;[1 1 1] Start_Joke02
  (bind _returnvalue (Audio|SpawnSound2D "/Game/Common/SFX/Player/SFX_Player_Joke02_Setup.SFX_Player_Joke02_Setup" 1.0 1.0 0.0 0 false false))
  (Components|Activation|SetActive _returnvalue true false)
  (Utilities|FlowControl|Delay 1.0)
  (bind _returnvalue_2 (Audio|SpawnSound2D "/Game/Common/SFX/Crowd/SFX_Crowd_Large_Applause.SFX_Crowd_Large_Applause" 1.0 1.0 0.0 0 false false))
  (Components|Activation|SetActive _returnvalue_2 true false)
  (bind _returnvalue_3 (Audio|SpawnSound2D "/Game/Common/SFX/Crowd/SFX_Crowd_Medium_Applause.SFX_Crowd_Medium_Applause" 1.0 1.0 0.0 0 false false))
  (Components|Activation|SetActive _returnvalue_3 true false)
  (Utilities|FlowControl|Delay 1e+01)
  (bind _returnvalue_4 (Audio|SpawnSound2D "/Game/Common/SFX/Player/SFX_Player_Joke01_Setup.SFX_Player_Joke01_Setup" 2.0 1.0 0.0 0))
  (Components|Activation|SetActive _returnvalue_4 true false)
  (Utilities|FlowControl|Delay 4.0))

(event EventBeginPlay
  ;[1 1 1] Debug
)

(fn ConstructionScript)