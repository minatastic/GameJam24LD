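; Collectible stress ball interactable that the player picks up through the Interact event.
; Overlapping InteractTrigger with a Player-tagged actor toggles custom depth on SMInteractable, marking the ball while in range.
; Interact spawns BP_StressFX at the trigger location and calls its OnSpawn, notifies LogicRef via OnCollect, then destroys the actor.
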(event OnComponentBeginOverlap(InteractTrigger)
  (params (OverlappedComponent :type Primitive%20Component%20Object%20Reference) (OtherActor :type Actor%20Object%20Reference) (OtherComp :type Primitive%20Component%20Object%20Reference) (OtherBodyIndex :type Integer) (bFromSweep :type Boolean) (SweepResult :type Hit%20Result%20Structure%20%28by%20ref%29))
  (if (Actor|ActorHasTag OtherActor "Player")
    (Rendering|SetRenderCustomDepth (Variables|Default|GetSM_Interactable) true)))

(event OnComponentEndOverlap(InteractTrigger)
  (params (OverlappedComponent :type Primitive%20Component%20Object%20Reference) (OtherActor :type Actor%20Object%20Reference) (OtherComp :type Primitive%20Component%20Object%20Reference) (OtherBodyIndex :type Integer))
  (if (Actor|ActorHasTag OtherActor "Player")
    (Rendering|SetRenderCustomDepth (Variables|Default|GetSM_Interactable) false)))

(event Custom|OnDestroyActor
  ;[1 1 1] Do stuff here
  (Actor|DestroyActor))

(event EventBeginPlay)

(event Collision|EventActorBeginOverlap
  (params (OtherActor :type Actor%20Object%20Reference)))

(event EventTick
  (params (DeltaSeconds :type Float%20%28single-precision%29)))

(event EventInteract
  ;[1 1 1] Do stuff here
  (bind _returnvalue (Game|SpawnActorfromClass "/Game/Common/Blueprints/BP_StressFX.BP_StressFX_C" (Math|Conversions|ToTransform(Vector) (Transformation|GetWorldLocation (Variables|Default|GetInteractTrigger))) "Undefined" 0 (Game|Player|GetPlayerPawn 0)))
  (Default|OnSpawn _returnvalue)
  (Default|OnCollect (Variables|Default|GetLogic_Ref))
  (CallFunction|OnDestroyActor))

(fn ConstructionScript
  (|CallParentFunction))