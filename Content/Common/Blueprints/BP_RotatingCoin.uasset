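; BP_RotatingCoin is a gold coin actor that spins around its vertical axis.
; On BeginPlay it waits a random delay of up to a few seconds, then plays the CoinRotation timeline, whose track sets the mesh's relative yaw.
; The random start offsets the rotation between coin instances.
; The construction script applies the Material variable to the coin mesh.
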(event EventBeginPlay
  (Variables|Default|SetDuration (Math|Random|RandomFloatinRange 0.0 4.0))
  (Utilities|FlowControl|RetriggerableDelay (Variables|Default|GetDuration))
  (bind _newtrack_0 (Timeline|CoinRotation Play)
    (:Update
      (Transformation|SetRelativeRotation (Variables|Default|GetSM_Gold_Coin) (Math|Rotator|MakeRotator 0.0 0.0 _newtrack_0) false false))))

(event Collision|EventActorBeginOverlap
  (params (OtherActor :type Actor%20Object%20Reference)))

(event EventTick
  (params (DeltaSeconds :type Float%20%28single-precision%29)))

(fn ConstructionScript
  (Rendering|Material|SetMaterial (Variables|Default|GetSM_Gold_Coin) 0 (Variables|Default|GetMaterial)))