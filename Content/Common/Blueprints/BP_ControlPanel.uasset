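; BP_ControlPanel is a decorative control panel prop with randomized indicator lights.
; Its construction script assigns each of five light material slots on the static mesh a random pick from lit, red and off material variants, so each placed panel can look different.
; The event graph is empty, so the panel has no runtime behavior of its own.
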(event EventBeginPlay)

(event Collision|EventActorBeginOverlap
  (params (OtherActor :type Actor%20Object%20Reference)))

(event EventTick
  (params (DeltaSeconds :type Float%20%28single-precision%29)))

(fn ConstructionScript
  (bind _staticmesh (Variables|Default|GetStaticMesh))
  (Rendering|Material|SetMaterial _staticmesh 4 (.OutItem (Utilities|Array|Random (Utilities|Array|MakeArray (Variables|Default|GetLight) (Variables|Default|GetLight2) (Variables|Default|GetLightRed) (Variables|Default|GetLightOff)))))
  (Rendering|Material|SetMaterial _staticmesh 5 (.OutItem (Utilities|Array|Random (Utilities|Array|MakeArray (Variables|Default|GetLight) (Variables|Default|GetLight2) (Variables|Default|GetLightRed) (Variables|Default|GetLightOff)))))
  (Rendering|Material|SetMaterial _staticmesh 6 (.OutItem (Utilities|Array|Random (Utilities|Array|MakeArray (Variables|Default|GetLight) (Variables|Default|GetLight2) (Variables|Default|GetLightRed) (Variables|Default|GetLightOff)))))
  (Rendering|Material|SetMaterial _staticmesh 7 (.OutItem (Utilities|Array|Random (Utilities|Array|MakeArray (Variables|Default|GetLight) (Variables|Default|GetLight2) (Variables|Default|GetLightRed) (Variables|Default|GetLightOff)))))
  (Rendering|Material|SetMaterial _staticmesh 8 (.OutItem (Utilities|Array|Random (Utilities|Array|MakeArray (Variables|Default|GetLight) (Variables|Default|GetLight2) (Variables|Default|GetLightRed) (Variables|Default|GetLightOff))))))