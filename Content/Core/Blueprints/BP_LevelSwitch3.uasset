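; Interactable level switch that moves the game on to the good or bad variant of the fourth venue level, depending on LogicRef.IsCleared.
; On Interact, either branch fades the camera and audio to black, plays a transition sound and opens the chosen level after a delay.
; A box overlap by a Player-tagged actor toggles custom depth on the Button as a highlight.
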(event OnComponentBeginOverlap(Box)
  (params (OverlappedComponent :type Primitive%20Component%20Object%20Reference) (OtherActor :type Actor%20Object%20Reference) (OtherComp :type Primitive%20Component%20Object%20Reference) (OtherBodyIndex :type Integer) (bFromSweep :type Boolean) (SweepResult :type Hit%20Result%20Structure%20%28by%20ref%29))
  (if (Actor|ActorHasTag OtherActor "Player")
    (Rendering|SetRenderCustomDepth (Variables|Default|GetButton) true)))

(event OnComponentEndOverlap(Box)
  (params (OverlappedComponent :type Primitive%20Component%20Object%20Reference) (OtherActor :type Actor%20Object%20Reference) (OtherComp :type Primitive%20Component%20Object%20Reference) (OtherBodyIndex :type Integer))
  (if (Actor|ActorHasTag OtherActor "Player")
    (Rendering|SetRenderCustomDepth (Variables|Default|GetButton) false)))

(event EventInteract
  (if (Variables|/Game/Core/Blueprints/BP_StressBall_Logic.BP_StressBall_Logic_C|GetisCleared (Variables|Default|GetLogic_Ref))
    (Utilities|FlowControl|Sequence
      (:then_0
        (CameraFades|StartCameraFade (Game|GetPlayerCameraManager 0) 0.0 1.0 3.0 "(R=0.000000,G=0.000000,B=0.000000,A=1.000000)" true true))
      (:then_1
        (Utilities|FlowControl|Delay 5.0)
        (Game|OpenLevel(byName) "LVL_Venue_4good"))
      (:then_2
        (AddComponent|AddAudioComponent false)
        (Audio|PlaySound2D "/Game/Common/SFX/Ambient/SFX_Ambient_TransitionSound01.SFX_Ambient_TransitionSound01" 1.0 1.0 0.0 0 0)))
    (else
      (Utilities|FlowControl|Sequence
        (:then_0
          (CameraFades|StartCameraFade (Game|GetPlayerCameraManager 0) 0.0 1.0 3.0 "(R=0.000000,G=0.000000,B=0.000000,A=1.000000)" true true))
        (:then_1
          (Utilities|FlowControl|Delay 5.0)
          (Game|OpenLevel(byName) "LVL_Venue_4bad"))
        (:then_2
          (AddComponent|AddAudioComponent false)
          (Audio|PlaySound2D "/Game/Common/SFX/Ambient/SFX_Ambient_TransitionSound01.SFX_Ambient_TransitionSound01" 1.0 1.0 0.0 0 0))))))

(fn ConstructionScript)